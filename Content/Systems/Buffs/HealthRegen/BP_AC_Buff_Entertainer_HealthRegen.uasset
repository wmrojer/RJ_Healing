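; Entertainer buff component that heals its owner over time, scaling regeneration by potency, stack size and a base regen value.
; The regen amount is recalculated on buff start and stack changes, before the parent logic runs.
; Each tick accumulates fractional regen and passes whole points to the parent's heal-over-time value, carrying the remainder.
; The description shows a separate replicated multiplier as a percentage, refreshing when it replicates.
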(event EventStartBuff
  (params (BuffPotency :type Integer) (DamageCauser :type Actor%20Object%20Reference) (OwningCharacter :type Conan%20Character%20Object%20Reference) (Instigator :type Controller%20Object%20Reference))
  (Variables|Default|SetCalculatedHealthRegen (CallFunction|CalculateHealthRegen))
  (|CallParentFunction BuffPotency DamageCauser OwningCharacter Instigator))

(event EventGameplayEffecttoApplyonBuffTick
  (bind _output_get (Variables|Default|SetAccumulatedHealthRegen (+ (Variables|Default|GetCalculatedHealthRegen) (Variables|Default|GetAccumulatedHealthRegen))))
  (if (> _output_get 1.0)
    (Variables|Default|SetHealOverTimeValue (Math|Float|Truncate _output_get))
    (Variables|Default|SetAccumulatedHealthRegen (- (Variables|Default|GetAccumulatedHealthRegen) (Math|Conversions|ToFloat(Integer) (Math|Float|Truncate _output_get))))
    (else
      (Variables|Default|SetHealOverTimeValue 0)))
  (|CallParentFunction))

(event EventAdjustStackSize
  (params (StackAdjustment :type Integer))
  (Variables|Default|SetCalculatedHealthRegen (CallFunction|CalculateHealthRegen))
  (|CallParentFunction StackAdjustment))

(fn CalculateHealthRegen
  (return (* (* (Variables|Default|GetBuffPotency) (Variables|Default|GetStackSize)) (Variables|Default|GetBuffHealthRegen))))

(fn GetEffectDescription
  (return (Utilities|Text|FormatText "Increase health regeneration by {RegenMultiplier}%." (Math|Float|Round (* (Variables|Default|GetCurrentHealthRegenMultiplier) 1e+02)))))

(fn OnRepCurrentHealthRegenMultiplier
  (Default|CallSignalEffectDescriptionChanged self))