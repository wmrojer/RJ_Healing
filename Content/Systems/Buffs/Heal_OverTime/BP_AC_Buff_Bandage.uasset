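; Bandage buff component, a heal-over-time effect in the buff system that also clears Crippled and weapon-proc Bleeding.
; StartBuff runs the parent start only on a BasePlayerChar without an active Bandage Large buff, then caches the owner's BuffSystem component.
; DoBuffTick defers to the parent tick and, when no ticks remain, ends both debuffs through that BuffSystem.
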(event EventStartBuff
  (params (BuffPotency :type Integer) (DamageCauser :type Actor%20Object%20Reference) (OwningCharacter :type Conan%20Character%20Object%20Reference) (Instigator :type Controller%20Object%20Reference))
  (bind _asbase_player_char (Utilities|Casting|CastToBasePlayerChar OwningCharacter))
  ;[1 1 1] Only apply if no Bandage Large is active
  (if (not (> (Utilities|Array|Length (Actor|GetComponentsByClass _asbase_player_char "/Game/Systems/Buffs/Heal_OverTime/BP_AC_Buff_Bandage_Large.BP_AC_Buff_Bandage_Large_C")) 0))
    (|CallParentFunction BuffPotency DamageCauser OwningCharacter Instigator)
    (Variables|Default|SetBuffSystem (Utilities|Array|Get(acopy) (Actor|GetComponentsByClass (Variables|Default|GetOwningCharacter) "/Game/Systems/Buffs/00_BP_AC_BuffSystem.00_BP_AC_BuffSystem_C")))))

(event EventDoBuffTick
  ;[1 1 1] Remove Cripple and Bleed on the last tick
  (|CallParentFunction)
  (if (== (Variables|Default|GetBuffTicks_Remaining) 0)
    (Default|EndBuff (Variables|Default|GetBuffSystem) "/Game/Systems/Buffs/Damage_OverTime/BP_AC_Buff_Crippled.BP_AC_Buff_Crippled_C")
    (Default|EndBuff (Variables|Default|GetBuffSystem) "/Game/Systems/Buffs/Damage_OverTime/BP_AC_Buff_Bleeding_WeaponProc.BP_AC_Buff_Bleeding_WeaponProc_C")))