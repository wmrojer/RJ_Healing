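; Large bandage buff component in the Heal_OverTime family that supersedes the regular bandage and clears injury debuffs on completion.
; On start it runs the parent logic, caches the owning character's buff system component and ends any regular Bandage buff.
; Each tick defers to the parent, and when no ticks remain it also ends the Crippled and weapon-proc Bleeding buffs.
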(event EventStartBuff
  (params (BuffPotency :type Integer) (DamageCauser :type Actor%20Object%20Reference) (OwningCharacter :type Conan%20Character%20Object%20Reference) (Instigator :type Controller%20Object%20Reference))
  (|CallParentFunction BuffPotency DamageCauser OwningCharacter Instigator)
  (bind _output_get (Variables|Default|SetBuffSystem (Utilities|Array|Get(acopy) (Actor|GetComponentsByClass (Variables|Default|GetOwningCharacter) "/Game/Systems/Buffs/00_BP_AC_BuffSystem.00_BP_AC_BuffSystem_C"))))
  ;[1 1 1] Remove lesser bandage buffs
  (Default|EndBuff _output_get "/Game/Systems/Buffs/Heal_OverTime/BP_AC_Buff_Bandage.BP_AC_Buff_Bandage_C"))

(event EventDoBuffTick
  ;[1 1 1] Remove Cripple and Bleed on the last tick
  (|CallParentFunction)
  (if (== (Variables|Default|GetBuffTicks_Remaining) 0)
    (Default|EndBuff (Variables|Default|GetBuffSystem) "/Game/Systems/Buffs/Damage_OverTime/BP_AC_Buff_Crippled.BP_AC_Buff_Crippled_C")
    (Default|EndBuff (Variables|Default|GetBuffSystem) "/Game/Systems/Buffs/Damage_OverTime/BP_AC_Buff_Bleeding_WeaponProc.BP_AC_Buff_Bleeding_WeaponProc_C")))