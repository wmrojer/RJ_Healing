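; Healing potion buff component that restores health over time to a player character.
; On start, it sets the per-tick heal to about a third of full max health divided by the buff's tick count.
; It skips the parent start logic if a Large Healing Potion buff is active; otherwise it starts, then on the server ends Hearty Meal and Small Potion healing buffs through the character's buff system.
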(event EventStartBuff
  (params (BuffPotency :type Integer) (DamageCauser :type Actor%20Object%20Reference) (OwningCharacter :type Conan%20Character%20Object%20Reference) (Instigator :type Controller%20Object%20Reference))
  (bind _asbase_player_char (Utilities|Casting|CastToBasePlayerChar OwningCharacter))
  ;[1 1 1] Calculate Heal Over Time as 33% of Health Max / Buff Ticks
  (Variables|Default|SetHealOverTimeValue (Math|Float|Truncate (/ (* (Class|ConanCharacter|GetIntStat _asbase_player_char "HealthMax" "Full") 0.33) (Math|Conversions|ToFloat(Integer) (Variables|/Game/Systems/Buffs/01_BP_AC_Buff_Master.01_BP_AC_Buff_Master_C|GetBuffTicks self)))))
  ;[1 1 1] Only apply buff if no Healing Potion Large is active
  (if (not (> (Utilities|Array|Length (Actor|GetComponentsByClass _asbase_player_char "/Game/Systems/Buffs/Heal_OverTime/BP_AC_Buff_HealingPotion_Large.BP_AC_Buff_HealingPotion_Large_C")) 0))
    (|CallParentFunction BuffPotency DamageCauser OwningCharacter Instigator)
    ;[1 1 1] End any active Healing HeartyMeal and Healing Potions Small buffs
    (bind _asbase_player_char_2 (Utilities|Casting|CastToBasePlayerChar (Variables|Default|GetOwningCharacter)))
    (if (Networking|IsServer)
      (Default|EndBuff (Variables|/Game/Characters/BaseBPCombat.BaseBPCombat_C|Get00_BP_AC_BuffSystem _asbase_player_char_2) "/Game/Systems/Buffs/Heal_OverTime/BP_AC_Buff_Healing_HeartyMeal.BP_AC_Buff_Healing_HeartyMeal_C")
      (Default|EndBuff (Variables|/Game/Characters/BaseBPCombat.BaseBPCombat_C|Get00_BP_AC_BuffSystem _asbase_player_char_2) "/Game/Systems/Buffs/Heal_OverTime/BP_AC_Buff_HealingPotion_Small.BP_AC_Buff_HealingPotion_Small_C"))))