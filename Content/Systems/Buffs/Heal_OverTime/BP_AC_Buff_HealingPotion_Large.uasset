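; Large healing potion buff component that heals the player over time for about two-thirds of their full max health.
; On start it derives a per-tick heal value from the max health stat and tick count, then passes to the parent buff's start logic.
; It then ends any active Hearty Meal, small and regular healing potion buffs through the player's buff system.
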(event EventStartBuff
  (params (BuffPotency :type Integer) (DamageCauser :type Actor%20Object%20Reference) (OwningCharacter :type Conan%20Character%20Object%20Reference) (Instigator :type Controller%20Object%20Reference))
  (bind _asbase_player_char (Utilities|Casting|CastToBasePlayerChar OwningCharacter))
  (Variables|Default|SetHealOverTimeValue (Math|Float|Truncate (/ (* (Class|ConanCharacter|GetIntStat _asbase_player_char "HealthMax" "Full") 0.66) (Math|Conversions|ToFloat(Integer) (Variables|/Game/Systems/Buffs/01_BP_AC_Buff_Master.01_BP_AC_Buff_Master_C|GetBuffTicks self)))))
  (|CallParentFunction BuffPotency DamageCauser OwningCharacter Instigator)
  ;[1 1 1] Remove any active HeartyMeal, Healing Potion Small and Healing Potion buffs
  (bind _asbase_player_char_2 (Utilities|Casting|CastToBasePlayerChar (Variables|Default|GetOwningCharacter)))
  (Default|EndBuff (Variables|/Game/Characters/BaseBPCombat.BaseBPCombat_C|Get00_BP_AC_BuffSystem _asbase_player_char_2) "/Game/Systems/Buffs/Heal_OverTime/BP_AC_Buff_Healing_HeartyMeal.BP_AC_Buff_Healing_HeartyMeal_C")
  (Default|EndBuff (Variables|/Game/Characters/BaseBPCombat.BaseBPCombat_C|Get00_BP_AC_BuffSystem _asbase_player_char_2) "/Game/Systems/Buffs/Heal_OverTime/BP_AC_Buff_HealingPotion_Small.BP_AC_Buff_HealingPotion_Small_C")
  (Default|EndBuff (Variables|/Game/Characters/BaseBPCombat.BaseBPCombat_C|Get00_BP_AC_BuffSystem _asbase_player_char_2) "/Game/Systems/Buffs/Heal_OverTime/BP_AC_Buff_HealingPotion.BP_AC_Buff_HealingPotion_C"))