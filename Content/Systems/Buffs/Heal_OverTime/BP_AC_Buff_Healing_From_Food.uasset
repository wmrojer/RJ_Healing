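; Healing buff component granted by food, deriving its heal-over-time strength from the potency passed in when the buff starts.
; On start it stores that potency as the heal value and defers to the parent buff logic.
; When the buff clears, it checks the owner's perk system component for Survivor_40 and, if present, applies an instant bonus heal scaled from the same value.
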(event EventStartBuff
  (params (BuffPotency :type Integer) (DamageCauser :type Actor%20Object%20Reference) (OwningCharacter :type Conan%20Character%20Object%20Reference) (Instigator :type Controller%20Object%20Reference))
  ;[1 1 1] Heal Over Time Value is set from the food that started the buff (max 1.0)
  (Variables|Default|SetHealOverTimeValue BuffPotency)
  (|CallParentFunction BuffPotency DamageCauser OwningCharacter Instigator))

(event EventGameplayEffecttoApplyonBuffCleared
  ;[1 1 1] Apply instant heal at end of buff if Perk Survivor_40 is active
  (bind _asbase_bpcombat (Utilities|Casting|CastToBaseBPCombat (Variables|Default|GetOwningCharacter)))
  (bind _asi_perk_system_interface (Utilities|Casting|CastToI_PerkSystemInterface (Actor|GetComponentbyClass (Variables|Default|GetOwningCharacter) "/Game/Systems/Perks/BP_PerkSystemComponent.BP_PerkSystemComponent_C")))
  (bind _hasperk (Default|HasPerk _asi_perk_system_interface "Survivor_40"))
  (if _hasperk
    (Default|AdjustHealth _asbase_bpcombat (Math|Float|Truncate (* (Variables|Default|GetHealOverTimeValue) 5.0)))))